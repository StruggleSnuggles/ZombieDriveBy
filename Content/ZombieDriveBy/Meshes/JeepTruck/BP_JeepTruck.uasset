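; BP_JeepTruck is the drivable jeep truck vehicle, with throttle, steering and an orbiting camera.
; Move axes feed the VehicleMovement component, while look axes rotate the SpringArm.
; Tick passes engine rotation speed to the engine sound's RPM parameter to drive its audio.
; Mesh hits play a collision sound at the impact point, throttled by a DoOnce that resets after a short delay.
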(event `InputAxis|LookUp`
  (params (AxisValue :type "Float (single-precision)"))
  ;[1 1 1] Camera
  (`SceneComponent.K2_AddRelativeRotation` (`self.SpringArm`) (`KismetMathLibrary.MakeRotator` 0.0 AxisValue) false false))

(event `InputAxis|MoveForward`
  (params (AxisValue :type "Float (single-precision)"))
  ;[1 1 1] vehicle move
  (`WheeledVehicleMovementComponent.SetThrottleInput` (`self.VehicleMovement`) AxisValue))

(event `InputAxis|LookRight`
  (params (AxisValue :type "Float (single-precision)"))
  ;[1 1 1] Camera
  (`SceneComponent.K2_AddRelativeRotation` (`self.SpringArm`) (`KismetMathLibrary.MakeRotator` 0.0 0.0 AxisValue) false false))

(event `InputAxis|MoveRight`
  (params (AxisValue :type "Float (single-precision)"))
  ;[1 1 1] vehicle move
  (`WheeledVehicleMovementComponent.SetSteeringInput` (`self.VehicleMovement`) AxisValue))

(event `self.ReceiveTick`
  (params (DeltaSeconds :type "Float (single-precision)"))
  ;[1 1 1] Sets engine rpm
  (`AudioComponent.SetFloatParameter` (`self.EngineSound`) "RPM" (`WheeledVehicleMovementComponent.GetEngineRotationSpeed` (`self.VehicleMovement`))))

(event `self.Mesh.OnComponentHit`
  (params (HitComponent :type "PrimitiveComponent Object Reference") (OtherActor :type "Actor Object Reference") (OtherComp :type "PrimitiveComponent Object Reference") (NormalImpulse :type "Vector Structure") (Hit :type "HitResult Structure (by ref)"))
  ;[1 1 1] play sound on collision
  (`/Engine/EditorBlueprintResources/StandardMacros.DoOnce` false :!label _label
    (:`Completed`
      (`GameplayStatics.PlaySoundAtLocation` "/Game/ZombieDriveBy/Sound/JeepTruck/Collision/A_RandomCollision.A_RandomCollision" (`.ImpactPoint` (`GameplayStatics.BreakHitResult` Hit)) (struct) 1.0 1.0 0.0 null null null)
      (`KismetSystemLibrary.Delay` 0.7)
      (goto _label :!via `Reset`))))

(fn `UserConstructionScript`)